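; Sliding door actor that opens when a ShooterCharacter interacts with it and closes when one leaves its Box trigger.
; Interacted and end overlap call the OpenDoor and CloseDoor events, which play open or close animations on the skeletal mesh; both callers also replay the same animation directly.
; Begin overlap does nothing, so proximity alone does not open the door, and a DoorOpening timeline is left unconnected.
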(event `self.Box.OnComponentBeginOverlap`
  (params (OverlappedComponent :type "PrimitiveComponent Object Reference") (OtherActor :type "Actor Object Reference") (OtherComp :type "PrimitiveComponent Object Reference") (OtherBodyIndex :type Integer) (bFromSweep :type Boolean) (SweepResult :type "HitResult Structure (by ref)")))

(event `/Game/Assets/Geometry/Meshes/Doors/Blueprints/InteractInterface.Interacted`
  (params (Interactor :type "Pawn Object Reference"))
  (cast `/Game/BaseGame/Blueprints/ShooterCharacter` Interactor)
  (`self.OpenDoor`)
  (`SkeletalMeshComponent.PlayAnimation` (`self.DoorMesh(Skeletal)`) "/Game/Assets/Geometry/Meshes/Doors/SlidingDoor/Door_Open_Door_Open.Door_Open_Door_Open" false))

(event `self.Box.OnComponentEndOverlap`
  (params (OverlappedComponent :type "PrimitiveComponent Object Reference") (OtherActor :type "Actor Object Reference") (OtherComp :type "PrimitiveComponent Object Reference") (OtherBodyIndex :type Integer))
  (cast `/Game/BaseGame/Blueprints/ShooterCharacter` OtherActor)
  (`self.CloseDoor`)
  (`SkeletalMeshComponent.PlayAnimation` (`self.DoorMesh(Skeletal)`) "/Game/Assets/Geometry/Meshes/Doors/SlidingDoor/Door_Open_Door_Close.Door_Open_Door_Close" false))

(event `OpenDoor`
  (`SkeletalMeshComponent.PlayAnimation` (`self.DoorMesh(Skeletal)`) "/Game/Assets/Geometry/Meshes/Doors/SlidingDoor/Door_Open_Door_Open.Door_Open_Door_Open" false))

(event `CloseDoor`
  (`SkeletalMeshComponent.PlayAnimation` (`self.DoorMesh(Skeletal)`) "/Game/Assets/Geometry/Meshes/Doors/SlidingDoor/Door_Open_Door_Close.Door_Open_Door_Close" false))

(fn `UserConstructionScript`)