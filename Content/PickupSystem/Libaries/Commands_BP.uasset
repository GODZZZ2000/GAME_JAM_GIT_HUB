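; Commands_BP is a pickup system helper library for finding interactable actors and showing prompt text.
; LineTrace traces the Visibility channel forward from a camera over a given sight distance, with optional debug drawing, and returns the hit actor only if it implements I_Interact_BP.
; PromptUser writes a supplied message into the PromptMessage text of a prompt widget.
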(fn `LineTrace`
  (params (Camera :type "CameraComponent Object Reference") (SightDistance :type "Float (double-precision)") (LineTraceDebug :type "EDrawDebugTrace Enum" :default "None"))
  (returns (HitActor :type "Actor Object Reference"))
  (bind _returnvalue (`SceneComponent.K2_GetComponentLocation` Camera))
  (bind (_outhit _returnvalue_2) (`KismetSystemLibrary.LineTraceSingle` :`WorldContextObject` Camera :`Start` _returnvalue :`End` (+ _returnvalue (* (`SceneComponent.GetForwardVector` Camera) SightDistance)) :`TraceChannel` "TraceTypeQuery1" :`DrawDebugType` LineTraceDebug))
  (if _returnvalue_2
    (bind (_bblockinghit _binitialoverlap _time _distance _location _impactpoint _normal _impactnormal _physmat _hitactor) (`GameplayStatics.BreakHitResult` _outhit))
    (if (`KismetSystemLibrary.DoesImplementInterface` _hitactor "/Game/Interface/I_Interact_BP.I_Interact_BP_C")
      (return _hitactor))))

(fn `PromptUser`
  (params (PromptWidgets :type "/Game/PickupSystem/Widgets/WBP_Prompt Object Reference") (PromptMessage :type Text))
  (`TextBlock.SetText` (`/Game/PickupSystem/Widgets/WBP_Prompt.PromptMessage` PromptWidgets) PromptMessage))