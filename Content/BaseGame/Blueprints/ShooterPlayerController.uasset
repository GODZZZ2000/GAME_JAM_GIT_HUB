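; ShooterPlayerController is a player controller that sets up the HUD and holds network test events for a multiplayer shooter.
; BeginPlay passes through RPC and multicast-named events to create the HeadsUpDisplay widget, then caches and prints player 0's ShooterCharacter.
; Tab triggers a debug scoreboard that prints each ShooterPlayerState's ID and score from the GameState's PlayerArray.
; A separate RPC test event increments a variable on ShooterGameState.
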(event `RPC_IncreaseVariable`
  ;[1 1 1] Network Button Test
  (bind _asshooter_game_state (cast `/Game/BaseGame/Blueprints/ShooterGameState` (`GameplayStatics.GetGameState`)))
  (`/Game/BaseGame/Blueprints/ShooterGameState.IncreaseVariable` _asshooter_game_state))

(event `self.ReceiveBeginPlay`
  ;[0.479 0.4766 0.75] Draw HUD for all Players
  (`self.RPC_DrawHUD`))

(event `RPC_DrawHUD`
  ;[0.479 0.4766 0.75] Draw HUD for all Players
  (`self.MC_DrawHUD`))

(event `MC_DrawHUD`
  ;[0.479 0.4766 0.75] Draw HUD for all Players
  (bind _returnvalue (`|CreateWidget` "/Game/BaseGame/UI/HeadsUpDisplay.HeadsUpDisplay_C"))
  (bind _output_get (set `self.HeadsUpDisplay` _returnvalue))
  (`UserWidget.AddToViewport` _output_get 0)
  (`|ExecutionSequence`
    (:`then_0`
      (bind _asshooter_character (cast `/Game/BaseGame/Blueprints/ShooterCharacter` (`GameplayStatics.GetPlayerCharacter` 0)))
      (bind _output_get_2 (set `self.TP_Char` _asshooter_character))
      (`KismetSystemLibrary.PrintString` (`KismetSystemLibrary.GetDisplayName` _output_get_2)))))

(event `Key|Tab`
  (params (Key :type "Key Structure"))
  ;[1 0.8328 0] Press TAB for Scoreboard
  (:`Pressed`
    (`self.RPC_DrawScores`)))

(event `RPC_DrawScores`
  ;[1 0.8328 0] Press TAB for Scoreboard
  (for _array_element (`GameStateBase.PlayerArray` (`GameplayStatics.GetGameState`))
    (bind _asshooter_player_state (cast `/Game/BaseGame/Blueprints/ShooterPlayerState` _array_element))
    (`KismetSystemLibrary.PrintString` (`KismetTextLibrary.Conv_TextToString` (`|FormatText` "Player ID: {id}        Score: {score}" (`PlayerState.PlayerId` _asshooter_player_state) (`/Game/BaseGame/Blueprints/ShooterPlayerState.PlayerScore` _asshooter_player_state))))))

(fn `UserConstructionScript`)