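; Player controller Blueprint that shows a simple debug-style scoreboard when Tab is pressed.
; The Tab press calls the RPC-named draw-scores event, which loops over the GameState's PlayerArray.
; Each entry is cast to ShooterPlayerState, and its player ID and score are formatted and output with PrintString, with no UI widget involved.
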(event `Key|Tab`
  (params (Key :type "Key Structure"))
  (:`Pressed`
    (`self.RPC_DrawScores`)))

(event `RPC_DrawScores`
  (for _array_element (`GameStateBase.PlayerArray` (`GameplayStatics.GetGameState`))
    (bind _asshooter_player_state (cast `/Game/BaseGame/Blueprints/ShooterPlayerState` _array_element))
    (`KismetSystemLibrary.PrintString` (`KismetTextLibrary.Conv_TextToString` (`|FormatText` "Player ID: {id}        Score: {score}" (`PlayerState.PlayerId` _asshooter_player_state) (`/Game/BaseGame/Blueprints/ShooterPlayerState.PlayerScore` _asshooter_player_state))))))

(fn `UserConstructionScript`)